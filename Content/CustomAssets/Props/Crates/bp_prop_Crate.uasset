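; Destructible Paper2D crate prop that breaks when its health is depleted by damage or when it is interacted with.
; Breaking disables physics and collision, plays the explode flipbook, spawns loot, then destroys the actor after the animation.
; The spawn macro randomly picks a weapon with paired ammo, though RandomInteger(3) never selects the Spitter case and large ammo is unwired.
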(event Custom|Destroyed
  (bind _crate (Variables|Default|Getcrate))
  (bind _crate_2 (Variables|Default|Getcrate))
  (Physics|SetSimulatePhysics (Variables|Default|Getcrate) false)
  (Collision|SetCollisionEnabled _crate_2 "NoCollision")
  (Sprite|SetFlipbook _crate_2 "/Game/CustomAssets/Props/Crates/Animations/crate_explode.crate_explode")
  (Utilities|SpawnItems)
  (Audio|Components|Audio|Play _crate)
  (Utilities|FlowControl|Delay (Class|PaperFlipbookComponent|GetFlipbookLength _crate))
  (Actor|DestroyActor))

(event EventDamage
  (params (amount :type Float%20%28single-precision%29) (damageCauser :type Actor%20Object%20Reference))
  (bind _output_get (Variables|Default|Sethealth (- (Variables|Default|Gethealth) amount)))
  (if (<= _output_get 0.0)
    (CallFunction|Destroyed)))

(event EventInteracted
  (params (playerReference :type Actor%20Object%20Reference) (controllerReference :type Actor%20Object%20Reference) (launch :type Boolean))
  (bind _crate (Variables|Default|Getcrate))
  (bind _crate_2 (Variables|Default|Getcrate))
  (Physics|SetSimulatePhysics (Variables|Default|Getcrate) false)
  (Collision|SetCollisionEnabled _crate_2 "NoCollision")
  (Sprite|SetFlipbook _crate_2 "/Game/CustomAssets/Props/Crates/Animations/crate_explode.crate_explode")
  (Utilities|SpawnItems)
  (Audio|Components|Audio|Play _crate)
  (Utilities|FlowControl|Delay (Class|PaperFlipbookComponent|GetFlipbookLength _crate))
  (Actor|DestroyActor))

(fn ConstructionScript)